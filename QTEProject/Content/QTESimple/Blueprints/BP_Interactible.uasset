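; BP_Interactible is a base interactable Blueprint with a toggleable InteractPrompt and start/end interaction state.
; Interact ignores calls while busy, otherwise sets IsBeingInteractedWith, fires InteractStarted and runs InteractionEvent.
; InteractionEvent is the hook for child Blueprints to override; its placeholder waits briefly, then EndInteract clears the flag and fires InteractEnded.
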(event Custom|ToggleInteractionPrompt
  (params (Show? :type Boolean))
  (Rendering|SetVisibility (Variables|Default|GetInteractPrompt) Show? false))

(event Custom|StartInteract
  (Variables|Default|SetbIsBeingInteractedWith true)
  (Default|CallInteractStarted))

(event Custom|EndInteract
  (Variables|Default|SetbIsBeingInteractedWith false)
  (Default|CallInteractEnded))

(event Custom|Interact
  (if (not (Variables|Default|GetbIsBeingInteractedWith))
    (CallFunction|StartInteract)
    (CallFunction|InteractionEvent)))

(event Custom|InteractionEvent
  ;[1 0.01729 0.09697] InteractionEvent is supposed to be overridden by child BPs. This is essentially the main function of this BP.
  ;;[1 1 1] What happens during interaction?
  (Utilities|FlowControl|Delay 5.0)
  (CallFunction|EndInteract))

(event EventBeginPlay)

(event Collision|EventActorBeginOverlap
  (params (OtherActor :type Actor%20Object%20Reference)))

(event EventTick
  (params (DeltaSeconds :type Float%20%28single-precision%29)))

(fn ConstructionScript)