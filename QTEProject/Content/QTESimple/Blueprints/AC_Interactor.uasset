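; Actor component that lets its owner find and interact with nearby BP_Interactible actors.
; Each tick it sphere-overlaps around the owner, keeps interactibles that allow interaction, picks the closest and updates its interaction prompt.
; InteractWithClosestInteractible binds to that target's start and end events and calls Interact.
; Those events disable further interaction until it ends, and prompt handling hides the prompt meanwhile.
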(event Custom|InteractWithInteractible
  (params (Interactible :type BP%20Interactible%20Object%20Reference))
  (Utilities|IsValid Interactible
    (:Is%20Valid
      (EventDispatchers|BindEventtoInteractStarted Interactible (EventDispatchers|CreateEvent :!event Custom|OnInteractStarted))
      (EventDispatchers|BindEventtoInteractEnded Interactible (EventDispatchers|CreateEvent :!event Custom|OntInteractEnded))
      (Default|Interact Interactible))
    (:Is%20Not%20Valid
      (Development|PrintString "INVALID INTERACTIBLE" true true "(R=1.000000,G=0.044178,B=0.000000,A=1.000000)" 15.0 ""))))

(event Custom|OnInteractStarted
  (Variables|Parameters|SetbCanInteractWithInteractibles false))

(event Custom|OntInteractEnded
  (Variables|Parameters|SetbCanInteractWithInteractibles true))

(event Custom|InteractWithClosestInteractible
  (bind (_hasinteractible_ _closestinteractible) (CallFunction|HasClosestInteractible))
  (if (Variables|Parameters|GetbCanInteractWithInteractibles)
    (if _hasinteractible_
      (CallFunction|InteractwithInteractible _closestinteractible)
      (else
        (Development|PrintString "There are no interactibles nearby." true true "(R=1.000000,G=0.000000,B=0.007579,A=1.000000)" 2.0 "")))
    (else
      (Development|PrintString "You can't interact with interactibles yet." true true "(R=1.000000,G=0.000000,B=0.007579,A=1.000000)" 2.0 ""))))

(event EventTick
  (params (DeltaSeconds :type Float%20%28single-precision%29))
  (bind _closestinteractible (CallFunction|GetClosestPotentialInteractible (CallFunction|GetAllPotentialInteractibles)))
  (CallFunction|HandleInteractiblePrompt _closestinteractible))

(fn GetAllPotentialInteractibles
  (bind _outactors (Collision|SphereOverlapActors (Transformation|GetActorLocation (Components|GetOwner self)) (Variables|Parameters|GetInteractionDistance) (Utilities|Array|MakeArray "ObjectTypeQuery2") "/Game/QTESimple/Blueprints/BP_Interactible.BP_Interactible_C"))
  (for _array_element _outactors
    (bind _asbp_interactible (Utilities|Casting|CastToBP_Interactible _array_element))
    (if (Variables|/Game/QTESimple/Blueprints/BP_Interactible.BP_Interactible_C|GetbCanBeInteractedWith _asbp_interactible)
      (Utilities|Array|AddUnique (LocalVariables|GetFoundInteractibles) _asbp_interactible)))
  (return (LocalVariables|GetFoundInteractibles)))

(fn GetClosestPotentialInteractible
  (params (PotentialInteractibles :type Array%20of%20BP%20Interactible%20Object%20References))
  (LocalVariables|SetClosestDistance 9999.0)
  (for _array_element PotentialInteractibles
    (if (< (Math|Vector|Distance(Vector) (Transformation|GetActorLocation (Components|GetOwner self)) (Transformation|GetActorLocation _array_element)) (LocalVariables|GetClosestDistance))
      (LocalVariables|SetClosestDistance (Math|Vector|Distance(Vector) (Transformation|GetActorLocation (Components|GetOwner self)) (Transformation|GetActorLocation _array_element)))
      (LocalVariables|SetChosenInteractible _array_element)))
  (return (LocalVariables|GetChosenInteractible)))

(fn HandleInteractiblePrompt
  (params (ClosestInteractible :type BP%20Interactible%20Object%20Reference))
  (if (Variables|Parameters|GetbCanInteractWithInteractibles)
    (if (and (!= (Variables|Interactibles|GetClosestInteractible) ClosestInteractible) (Utilities|IsValid (Variables|Interactibles|GetClosestInteractible)))
      (Default|ToggleInteractionPrompt (Variables|Interactibles|GetClosestInteractible) false))
    (bind _output_get (Variables|Interactibles|SetClosestInteractible ClosestInteractible))
    (Utilities|IsValid _output_get
      (:Is%20Valid
        (Default|ToggleInteractionPrompt _output_get true)))
    (elif (Utilities|IsValid (Variables|Interactibles|GetClosestInteractible))
      (Default|ToggleInteractionPrompt (Variables|Interactibles|GetClosestInteractible) false)
      (Variables|Interactibles|SetClosestInteractible 0))))

(fn HasClosestInteractible
  (bind _closestinteractible (Variables|Interactibles|GetClosestInteractible))
  (Utilities|IsValid _closestinteractible
    (:Is%20Valid
      (return true _closestinteractible))
    (:Is%20Not%20Valid
      (return false 0))))